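; Blueprint function library of general-purpose helpers for actor search, math, transforms, arrays and debug printing.
; Closest and furthest actor lookups linearly scan all actors of a class by distance from a start location.
; Increment and decrement helpers write through references, while array helpers build reversed or int/float-converted copies, with selectable rounding for float-to-int.
; GetRandomPointInRadius is an empty stub.
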(fn GetRandomPointinRadius)

(fn GetClosestActorOfClass
  (params (WorldContextObject :type Object%20Object%20Reference) (ActorClass :type Actor%20Class%20Reference) (StartLocation :type Vector))
  (bind _outactors (Actor|GetAllActorsOfClass WorldContextObject ActorClass))
  (for _array_element _outactors
    (if (< (Math|Vector|Distance(Vector) StartLocation (Transformation|GetActorLocation _array_element)) (LocalVariables|GetLocal_SmallestDistance))
      (LocalVariables|SetLocal_ClosestActor _array_element)
      (LocalVariables|SetLocal_SmallestDistance (Math|Vector|Distance(Vector) StartLocation (Transformation|GetActorLocation _array_element)))))
  (return (LocalVariables|GetLocal_ClosestActor) (LocalVariables|GetLocal_SmallestDistance)))

(fn GetFurthestActorOfClass
  (params (WorldContextObject :type Object%20Object%20Reference) (ActorClass :type Actor%20Class%20Reference) (StartLocation :type Vector))
  (bind _outactors (Actor|GetAllActorsOfClass WorldContextObject ActorClass))
  (for _array_element _outactors
    (if (> (Math|Vector|Distance(Vector) StartLocation (Transformation|GetActorLocation _array_element)) (LocalVariables|GetLocal_FurthestDistance))
      (LocalVariables|SetLocal_FurthestActor _array_element)
      (LocalVariables|SetLocal_FurthestDistance (Math|Vector|Distance(Vector) StartLocation (Transformation|GetActorLocation _array_element)))))
  (return (LocalVariables|GetLocal_FurthestActor) (LocalVariables|GetLocal_FurthestDistance)))

(fn IncrementFloat
  (params (Ref :type Float%20%28single-precision%29%20%28by%20ref%29) (Value :type Float%20%28single-precision%29))
  (bind _returnvalue (+ Ref Value))
  (|SetBy-RefVar Ref _returnvalue)
  (return _returnvalue))

(fn DecrementFloat
  (params (Ref :type Float%20%28single-precision%29%20%28by%20ref%29) (Value :type Float%20%28single-precision%29))
  (bind _returnvalue (- Ref Value))
  (|SetBy-RefVar Ref _returnvalue)
  (return _returnvalue))

(fn IncrementInt
  (params (Ref :type Integer) (Value :type Integer))
  (bind _returnvalue (+ Ref Value))
  (|SetBy-RefVar Ref _returnvalue)
  (return _returnvalue))

(fn DecrementInt
  (params (Ref :type Integer%20%28by%20ref%29) (Value :type Integer))
  (bind _returnvalue (- Ref Value))
  (|SetBy-RefVar Ref _returnvalue)
  (return _returnvalue))

(fn Float<0
  (params (InputFloat :type Float%20%28single-precision%29))
  (return (< InputFloat 0.0)))

(fn Float>0
  (params (InputFloat :type Float%20%28single-precision%29))
  (return (> InputFloat 0.0)))

(fn GetTransformLocation
  (params (InputTransform :type Transform))
  (return (.Location (Math|Transform|BreakTransform InputTransform))))

(fn GetTransformRotation
  (params (InputTransform :type Transform))
  (return (.Rotation (Math|Transform|BreakTransform InputTransform))))

(fn GetTransformScale
  (params (InputTransform :type Transform))
  (return (.Scale (Math|Transform|BreakTransform InputTransform))))

(fn PrintDebugMessage
  (params (Message :type String) (Prefix :type String) (Sufix :type String) (bPrintToScreen :type Boolean) (bPrintToLog :type Boolean) (TextColor :type Linear%20Color%20Structure :default "(R=0.000000,G=0.660000,B=1.000000,A=1.000000)") (Duration :type Float%20%28single-precision%29))
  (Development|PrintString 0 (Utilities|String|Append Prefix Message Sufix) bPrintToScreen bPrintToLog TextColor Duration))

(fn ReverseIntArray
  (params (InputArray :type Array%20of%20Integers))
  (bind _arrayelement (Utilities|Array|ReverseforEachLoop InputArray)
    (:LoopBody
      (Utilities|Array|Add (LocalVariables|GetLocal_IntArray) _arrayelement))
    (:Completed
      (return (LocalVariables|GetLocal_IntArray)))))

(fn ReverseFloatArray
  (params (InputArray :type Array%20of%20Floats%20%28single-precision%29))
  (bind _arrayelement (Utilities|Array|ReverseforEachLoop InputArray)
    (:LoopBody
      (Utilities|Array|Add (LocalVariables|GetLocal_IntArray) _arrayelement))
    (:Completed
      (return (LocalVariables|GetLocal_IntArray)))))

(fn ReverseVectorArray
  (params (InputArray :type Array%20of%20Vectors))
  (bind _arrayelement (Utilities|Array|ReverseforEachLoop InputArray)
    (:LoopBody
      (Utilities|Array|Add (LocalVariables|GetLocal_IntArray) _arrayelement))
    (:Completed
      (return (LocalVariables|GetLocal_IntArray)))))

(fn ArrayInttoFloat
  (params (InputArray :type Array%20of%20Integers))
  (for _array_element InputArray
    (Utilities|Array|Add (LocalVariables|GetLocal_FloatArray) (Math|Conversions|ToFloat(Integer) _array_element)))
  (return (LocalVariables|GetLocal_FloatArray)))

(fn ArrayFloattoInt
  (params (InputArray :type Array%20of%20Floats%20%28single-precision%29) (ConversionMethod :type Enum_FloatToIntConvertMethod%20Enum :default "NewEnumerator0"))
  (bind _local_floatarray (LocalVariables|GetLocal_FloatArray))
  (switch Utilities|FlowControl|Switch|SwitchonEnum_FloatToIntConvertMethod ConversionMethod
    (:NewEnumerator0
      (for _array_element InputArray
        (Utilities|Array|Add _local_floatarray (Math|Float|Truncate _array_element))))
    (:NewEnumerator1
      (for _array_element_2 InputArray
        (Utilities|Array|Add _local_floatarray (Math|Float|Round _array_element_2))))
    (:NewEnumerator2
      (for _array_element_3 InputArray
        (Utilities|Array|Add _local_floatarray (Math|Float|Ceil _array_element_3))))
    (:NewEnumerator3
      (for _array_element_4 InputArray
        (Utilities|Array|Add _local_floatarray (Math|Float|Floor _array_element_4)))))
  (return (LocalVariables|GetLocal_FloatArray)))